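; Dialogue component that runs branching, data-table-driven conversations in a dialogue widget.
; Each interaction shows the current row and stores the next row, table and end flag, closing the widget and restoring game input once ended.
; Open-ended rows spawn option buttons on opening or after a selection, each carrying its target row.
; On intro rows, player character tags override the row as icebreakers, then the tags and holding state are cleared.
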(event Custom|Option%20Selected
  (params (RowName :type Name) (DataTable :type Data%20Table%20Object%20Reference))
  (bind _returnvalue (Utilities|GetDataTableRow DataTable RowName)
    (:then
      (Widget|Panel|ClearChildren (Variables|/Game/Dialogue/WB_Dialogue.WB_Dialogue_C|GetOptionScrollBox (Variables|Default|GetDialogueWidget)))
      (Default|UpdateDialogue (Variables|Default|GetDialogueWidget) (.Dialogue (Utilities|Struct|BreakDialogue_Struct _returnvalue)))
      (Variables|Default|SetRow%20Name (.Row (Utilities|Struct|BreakDialogue_Struct _returnvalue)))
      (Variables|Default|SetData%20Table (.DataTable (Utilities|Struct|BreakDialogue_Struct _returnvalue)))
      (Variables|Default|SetEndDialogue (.EndDialogue (Utilities|Struct|BreakDialogue_Struct _returnvalue)))
      (if (.OpenEnded (Utilities|Struct|BreakDialogue_Struct _returnvalue))
        (for _array_element (.OpenEndedOptions (Utilities|Struct|BreakDialogue_Struct _returnvalue))
          (bind _returnvalue_2 (UserInterface|CreateWidget "/Game/Dialogue/WB_Options.WB_Options_C" 0 (Utilities|Text|ToText(Name) (.OptionName (Utilities|Struct|BreakOptionsDialogue_Struct _array_element))) self (.Row (Utilities|Struct|BreakOptionsDialogue_Struct _array_element)) (.DataTable (Utilities|Struct|BreakOptionsDialogue_Struct _array_element))))
          (Widget|Panel|AddChild (Variables|/Game/Dialogue/WB_Dialogue.WB_Dialogue_C|GetOptionScrollBox (Variables|Default|GetDialogueWidget)) _returnvalue_2))))))

(event Custom|Register%20Icebreaker
  (if (Utilities|Array|ContainsItem (Variables|Default|GetIntroOptions) (Variables|Default|GetRow%20Name))
    (bind _asbp_first_person_character (Utilities|Casting|CastToBP_FirstPersonCharacter (Game|GetPlayerCharacter 0)))
    (for _array_element (Variables|/Script/Engine.Actor|GetTags _asbp_first_person_character)
      (Variables|Default|SetRow%20Name _array_element)
      (Variables|/Script/Engine.Actor|SetTags _asbp_first_person_character (Variables|Default|GetEmptyArray))
      (Variables|/Game/FirstPerson/Blueprints/BP_FirstPersonCharacter.BP_FirstPersonCharacter_C|SetisHolding _asbp_first_person_character false))))

(event EventInteract
  (params (PlayerRef :type BP%20First%20Person%20Character%20Object%20Reference))
  (bind _returnvalue (Game|GetPlayerController 0))
  (bind _returnvalue_2 (Game|GetPlayerController 0))
  (CallFunction|RegisterIcebreaker)
  (if (Variables|Default|GetEndDialogue)
    (Widget|RemovefromParent (Variables|Default|GetDialogueWidget))
    (Variables|Default|SetEndDialogue false)
    (Variables|Default|SetDialogueWidget 0)
    (Input|SetInputModeGameOnly _returnvalue false)
    (Variables|/Script/Engine.PlayerController|SetbShowMouseCursor _returnvalue false)
    (else
      (Utilities|IsValid (Variables|Default|GetDialogueWidget)
        (:Is%20Valid
          (bind _returnvalue_3 (Utilities|GetDataTableRow (Variables|Default|GetData%20Table) (Variables|Default|GetRow%20Name))
            (:then
              (Default|UpdateDialogue (Variables|Default|GetDialogueWidget) (.Dialogue (Utilities|Struct|BreakDialogue_Struct _returnvalue_3)))
              (Variables|Default|SetRow%20Name (.Row (Utilities|Struct|BreakDialogue_Struct _returnvalue_3)))
              (Variables|Default|SetData%20Table (.DataTable (Utilities|Struct|BreakDialogue_Struct _returnvalue_3)))
              (Variables|Default|SetEndDialogue (.EndDialogue (Utilities|Struct|BreakDialogue_Struct _returnvalue_3))))))
        (:Is%20Not%20Valid
          (bind _returnvalue_4 (Utilities|GetDataTableRow (Variables|Default|GetData%20Table) (Variables|Default|GetRow%20Name))
            (:then
              (bind _returnvalue_5 (UserInterface|CreateWidget "/Game/Dialogue/WB_Dialogue.WB_Dialogue_C" 0 (Utilities|Text|ToText(Name) (Variables|Default|GetUserName)) (.Dialogue (Utilities|Struct|BreakDialogue_Struct _returnvalue_4))))
              (bind _output_get (Variables|Default|SetDialogueWidget _returnvalue_5))
              (UserInterface|Viewport|AddtoViewport _output_get 0)
              (Variables|Default|SetRow%20Name (.Row (Utilities|Struct|BreakDialogue_Struct _returnvalue_4)))
              (Variables|Default|SetData%20Table (.DataTable (Utilities|Struct|BreakDialogue_Struct _returnvalue_4)))
              (Variables|Default|SetEndDialogue (.EndDialogue (Utilities|Struct|BreakDialogue_Struct _returnvalue_4)))
              (Input|SetInputModeGameandUI _returnvalue_2 0 "DoNotLock" true false)
              (Variables|/Script/Engine.PlayerController|SetbShowMouseCursor _returnvalue_2 true)
              (if (.OpenEnded (Utilities|Struct|BreakDialogue_Struct _returnvalue_4))
                (for _array_element (.OpenEndedOptions (Utilities|Struct|BreakDialogue_Struct _returnvalue_4))
                  (bind _returnvalue_6 (UserInterface|CreateWidget "/Game/Dialogue/WB_Options.WB_Options_C" 0 (Utilities|Text|ToText(Name) (.OptionName (Utilities|Struct|BreakOptionsDialogue_Struct _array_element))) self (.Row (Utilities|Struct|BreakOptionsDialogue_Struct _array_element)) (.DataTable (Utilities|Struct|BreakOptionsDialogue_Struct _array_element))))
                  (Widget|Panel|AddChild (Variables|/Game/Dialogue/WB_Dialogue.WB_Dialogue_C|GetOptionScrollBox (Variables|Default|GetDialogueWidget)) _returnvalue_6))))))))))

(event EventLeaveDialogue
  (bind _returnvalue (Game|GetPlayerController 0))
  (Utilities|IsValid (Variables|Default|GetDialogueWidget)
    (:Is%20Valid
      (Widget|RemovefromParent (Variables|Default|GetDialogueWidget))
      (Variables|Default|SetEndDialogue false)
      (Variables|Default|SetDialogueWidget 0)
      (Input|SetInputModeGameOnly _returnvalue false)
      (Variables|/Script/Engine.PlayerController|SetbShowMouseCursor _returnvalue false))))