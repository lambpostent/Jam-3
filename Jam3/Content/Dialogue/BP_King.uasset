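; BP_King is a dialogue Blueprint for the King that switches its dialogue row based on the player character's state.
; Each Tick it casts the player to BP_FirstPersonCharacter and, while SpawnIcebreaker is set, checks ReadyToSelect.
; That flag selects the "Choose" row on BPDialogueComponent when true and "Icebreakers" when false, with a DoOnce on each branch so each assignment happens only once.
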(event EventTick
  (params (DeltaSeconds :type Float%20%28single-precision%29))
  (bind _asbp_first_person_character (Utilities|Casting|CastToBP_FirstPersonCharacter (Game|GetPlayerCharacter 0)))
  (if (Variables|/Game/FirstPerson/Blueprints/BP_FirstPersonCharacter.BP_FirstPersonCharacter_C|GetSpawnIcebreaker _asbp_first_person_character)
    (if (Variables|/Game/FirstPerson/Blueprints/BP_FirstPersonCharacter.BP_FirstPersonCharacter_C|GetReadyToSelect _asbp_first_person_character)
      (Utilities|FlowControl|DoOnce false
        (:Completed
          (Variables|/Game/Dialogue/BP_Dialogue_Component.BP_Dialogue_Component_C|SetRow%20Name (Variables|Default|GetBP_Dialogue_Component) "Choose")))
      (else
        (Utilities|FlowControl|DoOnce false
          (:Completed
            (Variables|/Game/Dialogue/BP_Dialogue_Component.BP_Dialogue_Component_C|SetRow%20Name (Variables|Default|GetBP_Dialogue_Component) "Icebreakers")))))))

(fn ConstructionScript)