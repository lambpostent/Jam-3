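; BP_NPC is a dialogue NPC that reports to the player character when its conversation reaches an intro or ice option.
; Each Tick it checks its dialogue component's current RowName against the IntroOptions list, then against IceOptions if that fails.
; A separate DoOnce per category limits each NPC to one IncrementIntros and one IncrementIce call on BP_FirstPersonCharacter, with no reset shown.
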(event EventTick
  (params (DeltaSeconds :type Float%20%28single-precision%29))
  (if (Utilities|Array|ContainsItem (Variables|Default|GetIntroOptions) (Variables|/Game/Dialogue/BP_Dialogue_Component.BP_Dialogue_Component_C|GetRow%20Name (Variables|Default|GetBP_Dialogue_Component)))
    (Utilities|FlowControl|DoOnce false
      (:Completed
        (bind _asbp_first_person_character (Utilities|Casting|CastToBP_FirstPersonCharacter (Game|GetPlayerCharacter 0)))
        (Default|IncrementIntros _asbp_first_person_character)))
    (elif (Utilities|Array|ContainsItem (Variables|Default|GetIceOptions) (Variables|/Game/Dialogue/BP_Dialogue_Component.BP_Dialogue_Component_C|GetRow%20Name (Variables|Default|GetBP_Dialogue_Component)))
      (Utilities|FlowControl|DoOnce false
        (:Completed
          (bind _asbp_first_person_character_2 (Utilities|Casting|CastToBP_FirstPersonCharacter (Game|GetPlayerCharacter 0)))
          (Default|IncrementIce _asbp_first_person_character_2))))))

(fn ConstructionScript)