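; BP_CountessBizzyBoday is the dialogue character actor for Countess Bizzy Boday, tracking whether she is the one the player is talking to.
; It caches the first-person player on BeginPlay and polls its IsInteracting flag on Tick, with a DoOnce that resets when interaction ends.
; Once per interaction, SelectAnim sets IsTalking by comparing its own object name to the player's InteractActorName, with an optional debug print.
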(event EventTick
  (params (DeltaSeconds :type Float%20%28single-precision%29))
  (if (Variables|/Game/FirstPerson/Blueprints/BP_FirstPersonCharacter.BP_FirstPersonCharacter_C|GetIsInteracting (Variables|Default|GetPlayerBP))
    (Utilities|FlowControl|DoOnce false :!label _label
      (:Completed
        (CallFunction|SelectAnim)))
    (else
      (goto _label Reset))))

(event EventBeginPlay
  (bind _returnvalue (Actor|GetActorOfClass "/Game/FirstPerson/Blueprints/BP_FirstPersonCharacter.BP_FirstPersonCharacter_C"))
  (Variables|Default|SetPlayerBP _returnvalue))

(fn ConstructionScript)

(fn SelectAnim
  (if (Utilities|Enum|Equal(Enum) (Utilities|GetObjectName self) (Variables|/Game/FirstPerson/Blueprints/BP_FirstPersonCharacter.BP_FirstPersonCharacter_C|GetInteractActor%20Name (Variables|Default|GetPlayerBP)))
    (bind _output_get (Variables|Default|SetIsTalking true))
    (else
      (Variables|Default|SetIsTalking false)))
  (if (Variables|Default|GetDEBUGis%20Talking)
    (Development|PrintString (Utilities|String|ToString(Boolean) _output_get))))