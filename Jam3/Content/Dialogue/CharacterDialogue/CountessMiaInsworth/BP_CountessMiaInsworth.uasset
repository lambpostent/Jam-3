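; Dialogue NPC Countess Mia Insworth, which tracks when the player is talking to her and reports dialogue milestones.
; Each Tick, it checks the dialogue component's current row against intro and ice option lists, incrementing the matching player counter once each.
; When player interaction starts, a resettable DoOnce runs SelectAnim, setting IsTalking by comparing her object name to the player's InteractActorName, with optional debug printing.
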(event Custom|IncrementSteps
  (if (Utilities|Array|ContainsItem (Variables|Default|GetIntroOptions) (Variables|/Game/Dialogue/BP_Dialogue_Component.BP_Dialogue_Component_C|GetRow%20Name (Variables|Default|GetBP_Dialogue_Component)))
    (Utilities|FlowControl|DoOnce false
      (:Completed
        (bind _asbp_first_person_character (Utilities|Casting|CastToBP_FirstPersonCharacter (Game|GetPlayerCharacter 0)))
        (Default|IncrementIntros _asbp_first_person_character)))
    (elif (Utilities|Array|ContainsItem (Variables|Default|GetIceOptions) (Variables|/Game/Dialogue/BP_Dialogue_Component.BP_Dialogue_Component_C|GetRow%20Name (Variables|Default|GetBP_Dialogue_Component)))
      (Utilities|FlowControl|DoOnce false
        (:Completed
          (bind _asbp_first_person_character_2 (Utilities|Casting|CastToBP_FirstPersonCharacter (Game|GetPlayerCharacter 0)))
          (Default|IncrementIce _asbp_first_person_character_2))))))

(event EventTick
  (params (DeltaSeconds :type Float%20%28single-precision%29))
  (CallFunction|IncrementSteps)
  (if (Variables|/Game/FirstPerson/Blueprints/BP_FirstPersonCharacter.BP_FirstPersonCharacter_C|GetIsInteracting (Variables|Default|GetPlayerBP))
    (Utilities|FlowControl|DoOnce false :!label _label
      (:Completed
        (CallFunction|SelectAnim)))
    (else
      (goto _label Reset))))

(event EventBeginPlay
  (bind _returnvalue (Actor|GetActorOfClass "/Game/FirstPerson/Blueprints/BP_FirstPersonCharacter.BP_FirstPersonCharacter_C"))
  (Variables|Default|SetPlayerBP _returnvalue))

(fn ConstructionScript)

(fn SelectAnim
  (if (Utilities|Enum|Equal(Enum) (Utilities|GetObjectName self) (Variables|/Game/FirstPerson/Blueprints/BP_FirstPersonCharacter.BP_FirstPersonCharacter_C|GetInteractActor%20Name (Variables|Default|GetPlayerBP)))
    (bind _output_get (Variables|Default|SetIsTalking true))
    (else
      (Variables|Default|SetIsTalking false)))
  (if (Variables|Default|GetDEBUGis%20Talking)
    (Development|PrintString (Utilities|String|ToString(Boolean) _output_get))))