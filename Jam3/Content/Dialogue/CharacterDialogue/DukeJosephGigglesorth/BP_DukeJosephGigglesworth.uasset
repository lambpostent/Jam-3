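; Duke Joseph Gigglesworth dialogue character that sets talking and idle animation flags from the player's interaction state.
; Tick runs SelectAnim once per interaction, and the player leaving the capsule overlap clears talking and reruns it.
; SelectAnim acts only when this actor's name matches the player's interaction target, randomly picking one of two idle poses when not talking.
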(event OnComponentEndOverlap(CapsuleComponent)
  (params (OverlappedComponent :type Primitive%20Component%20Object%20Reference) (OtherActor :type Actor%20Object%20Reference) (OtherComp :type Primitive%20Component%20Object%20Reference) (OtherBodyIndex :type Integer))
  (if (Utilities|Enum|Equal(Enum) (Utilities|GetObjectName OtherActor) (Utilities|GetObjectName (Variables|Default|GetPlayerBP)))
    (Variables|Default|SetIsTalking false)
    (CallFunction|SelectAnim)))

(event EventTick
  (params (DeltaSeconds :type Float%20%28single-precision%29))
  (if (Variables|/Game/FirstPerson/Blueprints/BP_FirstPersonCharacter.BP_FirstPersonCharacter_C|GetIsInteracting (Variables|Default|GetPlayerBP))
    (Utilities|FlowControl|DoOnce false :!label _label
      (:Completed
        (CallFunction|SelectAnim)))
    (else
      (goto _label Reset))))

(event EventBeginPlay
  (bind _returnvalue (Actor|GetActorOfClass "/Game/FirstPerson/Blueprints/BP_FirstPersonCharacter.BP_FirstPersonCharacter_C"))
  (Variables|Default|SetPlayerBP _returnvalue))

(fn ConstructionScript)

(fn SelectAnim
  (bind _playerbp (Variables|Default|GetPlayerBP))
  (if (Utilities|Enum|Equal(Enum) (Utilities|GetObjectName self) (Variables|/Game/FirstPerson/Blueprints/BP_FirstPersonCharacter.BP_FirstPersonCharacter_C|GetInteractActor%20Name _playerbp))
    (if (Variables|/Game/FirstPerson/Blueprints/BP_FirstPersonCharacter.BP_FirstPersonCharacter_C|GetIsInteracting _playerbp)
      (bind _output_get (Variables|Default|SetIsTalking true))
      (Variables|Default|SetIsIdle false)
      (else
        (bind _output_get_2 (Variables|Default|SetIsTalking false))))
    (if (Variables|Default|GetDEBUGis%20Talking)
      (Development|PrintString (Utilities|String|ToString(Boolean) _output_get) true true "(R=0.282136,G=1.000000,B=0.301904,A=1.000000)"))
    (if _output_get_2
      (Variables|Default|SetIsIdle false)
      (else
        (Variables|Default|SetIsIdle true)
        (bind _output_number (CallFunction|SelectRandomNumber))
        (if (== _output_number 1)
          (Variables|Default|SetDoIdlePose2 false)
          (Variables|Default|SetDoIdlePose1 true)
          (else
            (Variables|Default|SetDoIdlePose1 false)
            (Variables|Default|SetDoIdlePose2 true)))))))

(fn SelectRandomNumber
  (bind _output_get (Variables|Default|SetReturnINT (Math|Random|RandomIntegerinRange 1 2)))
  (if (Variables|Default|GetDEBUG%20INT)
    (Development|PrintString (Utilities|String|ToString(Integer) _output_get) true true "(R=0.877693,G=1.000000,B=0.047679,A=1.000000)"))
  (return _output_get))