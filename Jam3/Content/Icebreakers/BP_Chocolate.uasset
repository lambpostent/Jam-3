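; BP_Chocolate is a chocolate pickup, one of the icebreaker items the first-person character can hold.
; It starts hidden with collision off, then polls the player's SpawnIcebreaker flag on Tick and shows itself with collision restored while that flag is true.
; On overlap with a player who is not holding anything, it sets IsHolding, replaces the character's Tags with its own and destroys itself.
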(event Custom|EnableObject
  (Development|SetHiddeninGame (Variables|Default|GetDefaultSceneRoot) false true)
  (Collision|SetCollisionEnabled (Variables|Default|GetBox) "QueryAndPhysics")
  (Collision|SetCollisionEnabled (Variables|Default|GetCube) "QueryAndPhysics"))

(event Custom|DisableObject
  (Development|SetHiddeninGame (Variables|Default|GetDefaultSceneRoot) true true)
  (Collision|SetCollisionEnabled (Variables|Default|GetBox) "NoCollision")
  (Collision|SetCollisionEnabled (Variables|Default|GetCube) "NoCollision"))

(event EventBeginPlay
  (CallFunction|DisableObject))

(event EventTick
  (params (DeltaSeconds :type Float%20%28single-precision%29))
  (bind _asbp_first_person_character (Utilities|Casting|CastToBP_FirstPersonCharacter (Game|GetPlayerCharacter 0)))
  (if (Variables|/Game/FirstPerson/Blueprints/BP_FirstPersonCharacter.BP_FirstPersonCharacter_C|GetSpawnIcebreaker _asbp_first_person_character)
    (CallFunction|EnableObject)))

(event Collision|EventActorBeginOverlap
  (params (OtherActor :type Actor%20Object%20Reference))
  (bind _asbp_first_person_character (Utilities|Casting|CastToBP_FirstPersonCharacter OtherActor))
  (if (not (Variables|/Game/FirstPerson/Blueprints/BP_FirstPersonCharacter.BP_FirstPersonCharacter_C|GetisHolding _asbp_first_person_character))
    (Variables|/Game/FirstPerson/Blueprints/BP_FirstPersonCharacter.BP_FirstPersonCharacter_C|SetisHolding _asbp_first_person_character true)
    (Variables|/Script/Engine.Actor|SetTags _asbp_first_person_character (Variables|Actor|GetTags))
    (Actor|DestroyActor)))

(fn ConstructionScript)